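; Master enemy AI Blueprint that activates the enemy when the player enters its trigger box.
; BeginPlay casts and caches its BP_master_AI_controller.
; When player character 0 begins overlapping the Box, it sets the Is_Enmey_Active blackboard bool to true through that controller, and nothing here resets it.
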(event `self.ReceiveBeginPlay`
  ;[1 1 1] cast Enmy AI controllier
  (bind _asbp_master_ai_controller (cast `/Game/Sayaf_project/MasterAI/BP_master_AI_controller` (`AIBlueprintHelperLibrary.GetAIController` self)))
  (set `self.As BP Master AI Controller` _asbp_master_ai_controller))

(event `self.Box.OnComponentBeginOverlap`
  (params (OverlappedComponent :type "PrimitiveComponent Object Reference") (OtherActor :type "Actor Object Reference") (OtherComp :type "PrimitiveComponent Object Reference") (OtherBodyIndex :type Integer) (bFromSweep :type Boolean) (SweepResult :type "HitResult Structure (by ref)"))
  ;[0.1458 0.1086 0.09534] Enemy activation
  ;;[1 1 1] Check if is player
  (if (== OtherActor (`GameplayStatics.GetPlayerCharacter` 0))
    ;;[1 1 1] set BB bool true
    (`BlackboardComponent.SetValueAsBool` (`AIBlueprintHelperLibrary.GetBlackboard` (`self.As BP Master AI Controller`)) "Is_Enmey_Active" true)))

(fn `UserConstructionScript`)